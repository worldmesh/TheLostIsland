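; BP_Generator is an interactable generator in The Lost Island that the player switches on and off.
; Interact advances CurrentState from its first value to the second, then toggles between the second and third on later uses.
; After each change it tells the player's BP_ThirdPersonCharacter to refresh the interaction widget.
; BeginPlay and construction only call the parent, and Tick is disabled.
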(event `self.ReceiveBeginPlay`
  (`parent.ReceiveBeginPlay`))

(event `self.Interact`
  ; Генератор вкл/выкл
  (bind _asbp_third_person_character (cast `/Game/ThirdPerson/Blueprints/BP_ThirdPersonCharacter` (`GameplayStatics.GetPlayerCharacter` 0)))
  (if (== (`self.CurrentState`) 1)
    (`self.SetCurrentState` 2)
    (`TheLostIslandCharacter.RefreshInteractionWidget` _asbp_third_person_character)
    (else
      (switch `int` (`self.CurrentState`)
        (:`2`
          (`self.SetCurrentState` 3)
          (`TheLostIslandCharacter.RefreshInteractionWidget` _asbp_third_person_character))
        (:`3`
          (`self.SetCurrentState` 2)
          (`TheLostIslandCharacter.RefreshInteractionWidget` _asbp_third_person_character))))))

(fn `UserConstructionScript`
  (`parent.UserConstructionScript`))