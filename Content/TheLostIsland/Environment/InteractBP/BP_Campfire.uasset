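; BP_Campfire is an interactable campfire actor whose point light can be switched on and off.
; BeginPlay starts with the light at zero intensity, and Interact drives a small state machine on CurrentState.
; The first state advances to the second without changing the light; later interactions alternate between the second and third states, lighting and extinguishing it.
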(event `self.ReceiveBeginPlay`
  (`parent.ReceiveBeginPlay`)
  (`LightComponent.SetIntensity` (`self.PointLight`) 0.0))

(event `self.Interact`
  (switch `int` (`self.CurrentState`)
    (:`1`
      (`self.SetCurrentState` 2))
    (:`2`
      (`self.SetCurrentState` 3)
      (`LightComponent.SetIntensity` (`self.PointLight`) 20000.0))
    (:`3`
      (`self.SetCurrentState` 2)
      (`LightComponent.SetIntensity` (`self.PointLight`) 0.0))))

(fn `UserConstructionScript`
  (`parent.UserConstructionScript`))