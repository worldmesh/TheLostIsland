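; BP_ReportObject is an overlap-triggered actor that briefly shows an interaction prompt about a linked target object.
; On any actor overlap, it checks whether TargetObject's current state matches RequiredState.
; If so, it creates a WBP_Interaction widget from the target's display name and action text, updates it, adds it to the viewport and removes it after a short delay.
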(event `self.ReceiveActorBeginOverlap`
  (params (OtherActor :type "Actor Object Reference"))
  (bind _targetobject (`self.TargetObject`))
  (if (== (`WorldObject.CurrentState` (`self.TargetObject`)) (`self.RequiredState`))
    (bind _returnvalue (`|CreateWidget` "/Game/TheLostIsland/Content/UI/WBP_Interaction.WBP_Interaction_C" null (`WorldObject.DisplayName` _targetobject) (`self.GetActionText` _targetobject)))
    (bind _output_get (set `self.WBP_Widget_Ref` _returnvalue))
    (`/Game/TheLostIsland/Content/UI/WBP_Interaction.UpdateInteraction` _output_get)
    (`UserWidget.AddToViewport` _output_get 0)
    (`KismetSystemLibrary.Delay` 1.5)
    (`Widget.RemoveFromParent` (`self.WBP_Widget_Ref`))))

(fn `UserConstructionScript`
  (`parent.UserConstructionScript`))